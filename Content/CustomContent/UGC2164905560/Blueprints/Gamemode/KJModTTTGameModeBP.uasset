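; Server-side game mode for a Trouble in Terrorist Town (TTT) round of innocents, detectives and traitors.
; A one-second timer drives a state machine through waiting, pregame, spawn lockout, role selection, main round, winner report and reset.
; Each joiner gets a KJModTTTPlayerBP proxy that receives its randomly drawn role, phase times and messages.
; Deaths and departures update an alive list that decides the winner; innocents win on timeout.
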(event Custom|StateMachineEvent
  ;[0.2965 1 0.1402] BEGIN PLAY - Process state machine every second
  (switch Utilities|FlowControl|Switch|SwitchonKJModTTTGameStateEnum (Variables|GameState|GetState)
    (:NewEnumerator2
      (StateManagement|HandleWaitingonEnoughPlayersState) ; Just waiting for players > X
    )
    (:NewEnumerator3
      (StateManagement|HandlePregameState) ; Players can join at this point, other's just wait around 'preparing'
      ;;[1 0.468 0.2456 1 12] Only certain states we care about this..
      (StateManagement|CheckEnoughPlayers))
    (:NewEnumerator8
      (StateManagement|HandlePregameLockoutState) ; Used to prevent users from joining just before we kick off everything (5 seconds)
      (StateManagement|CheckEnoughPlayers))
    (:NewEnumerator4
      (StateManagement|HandleSelectionState) ; Make a traitor or two.. moves straight on to Main phase
    )
    (:NewEnumerator5
      (StateManagement|HandleMainPhase) ; Go find some traitors!
      (StateManagement|CheckEnoughPlayers))
    (:NewEnumerator6
      (StateManagement|HandleWinnerPhase) ; One side is dead (or everyone is dead!)
    )
    (:NewEnumerator7
      (StateManagement|HandleGameReset) ; Reset for next round
    )))

(event Custom|PlayerHasDied
  (params (DeadPlayer :type KJ%20Mod%20TTT%20Player%20BP%20Object%20Reference))
  ;[1 1 1] PLAYER DIED - Handle their death
  (PlayerManagement|HandlePlayerDeath DeadPlayer))

(event EventBeginPlay
  ;[0.2965 1 0.1402] BEGIN PLAY - Process state machine every second
  (Utilities|Time|SetTimerbyEvent (delegate Custom|StateMachineEvent) 1.0 true) ; Set up our 1 second timer to look after states
)

(event EventGameModeActivated
  ;[1 0.8675 0.1036] GAME MODE ACTIVATED EVENT
  ;;[1 1 1] Always spawn our players as spectators initially, we will make them full players later
  (Class|KJModGameModeProxy|SetJoiningPlayersParameters (Utilities|Struct|MakeKJModGameModeProxyPlayerJoinParameters true 0.0 false 5.0 0.0))
  ;;[1 1 1] Start the states by resetting state machine
  (StateManagement|SwitchtoNewState "NewEnumerator7"))

(fn ConstructionScript)

(fn PlayerHasJoined
  (params (joiningPlayerController :type Player%20Controller%20Object%20Reference))
  ;[1 1 1] SERVER - Handle player joining
  (Variables|GameState|SetCurrentPlayerCount (+ (Variables|GameState|GetCurrentPlayerCount) 1))
  (CallFunction|PrintDebugMessage "[Mod] Player Has Joined" "(R=0.000000,G=1.000000,B=0.038267,A=1.000000)" 5.0)
  ;[1 1 1] Spawn the TTT player proxy (i.e. player representation)
  (bind _returnvalue (Game|SpawnActorfromClass "/Game/CustomContent/UGC2164905560/Blueprints/PlayerRepresentation/KJModTTTPlayerBP.KJModTTTPlayerBP_C" (Math|Transform|MakeTransform "0, 0, 0") "Undefined" joiningPlayerController self 0)) ; Note: As we run on server, we set owner of the player representation to the new controller (for "Execute On Owning Client" Events sent to it)
  ;[1 1 1] Record it, and initialise it with the related player controller
  (Utilities|Array|Add (Variables|PlayerRepresentations|GetTTTPlayerRepresentation) _returnvalue) ; Record it, so we can destroy it later
  (Class|KJModPlayerProxy|Initialise _returnvalue joiningPlayerController self (Utilities|Struct|MakeKJModPlayerProxyPawnSettings 100 0 false true true)) ; Must call initialise after spawning, must include player controller
  ;[0.6744 1 0.9601] Has the player joined in a state where they should immediately spawn?
  (if (Utilities|Select :Index (Variables|GameState|GetState) :NewEnumerator0 true :NewEnumerator2 true :NewEnumerator3 true :NewEnumerator8 false :NewEnumerator4 false :NewEnumerator5 false :NewEnumerator6 false :NewEnumerator7 true)
    (Class|KJModGameModeProxy|SpawnPlayer _returnvalue) ; Note: As we have set up this GM to have joining players as spectators this will take a full second FULL SECOND to spawn the real player pawn.
  )
  (return _returnvalue))

(fn PrintDebugMessage
  (params (Message :type String) (COlor :type Linear%20Color%20Structure) (TTL :type Float%20%28single-precision%29))
  ;[1 1 1] We use the Print Debug Message in the Proxy, UE4 doesn't support "PrintString" at run-time in shipping games
  (if (Variables|ModConfig|GetShouldDebugPrintGameMode)
    (Class|KJModProxy|PrintStringKJMod 0 Message true true COlor TTL)
    (Development|PrintString Message true true COlor TTL)))

(fn HandlePregameState
  (CallFunction|PrintDebugMessage (Utilities|String|Append "[Mod State] Pregame state, timeout: " (Utilities|String|ToString(Integer) (Variables|GameState-Pregame|GetPregameTimeout))) "(R=0.088961,G=0.651042,B=0.000000,A=1.000000)" 5.0)
  (bind _result (Math|Integer|DecrementInt (Variables|GameState-Pregame|GetPregameTimeout))
    (:%20%20
      (bind _output_get (Variables|GameState-Pregame|SetPregameTimeout _result))
      (if (== _output_get 0)
        (StateManagement|SwitchtoNewState "NewEnumerator8")))))

(fn HandleWaitingonEnoughPlayersState
  (if (>= (Variables|GameState|GetCurrentPlayerCount) (Variables|GameSettings(Editthese)|GetMinPlayers))
    ;[1 1 1] Enough players have arrived, move on (reset flags too)
    (CallFunction|ShowInformationtoAllPlayers false)
    (StateManagement|SwitchtoNewState "NewEnumerator3")
    (Variables|GameState-WaitingOnPlayers|SetWaitingOnPlayersTime 0)
    (else
      ;[1 1 1] If waiting, show information to clients
      (bind _output_get (Variables|GameState-WaitingOnPlayers|SetWaitingOnPlayersTime (+ (Variables|GameState-WaitingOnPlayers|GetWaitingOnPlayersTime) 1)))
      (CallFunction|ShowInformationtoAllPlayers true (Utilities|String|Append "Waiting on more players (require " (Utilities|String|ToString(Integer) (Variables|GameSettings(Editthese)|GetMinPlayers)) " players) - " (Utilities|String|Right (Utilities|String|Append "0" (Utilities|String|ToString(Integer) (.Minutes (Math|Timespan|BreakTimespan (Math|Timespan|MakeTimespan 0 0 0 _output_get))))) 2) ":" (Utilities|String|Right (Utilities|String|Append "0" (Utilities|String|ToString(Integer) (.Seconds (Math|Timespan|BreakTimespan (Math|Timespan|MakeTimespan 0 0 0 _output_get))))) 2))))))

(fn PlayerHasLeft
  (params (leavingPlayerController :type Player%20Controller%20Object%20Reference))
  ;[1 1 1] Reduce active player counts
  (Variables|GameState|SetCurrentPlayerCount (- (Variables|GameState|GetCurrentPlayerCount) 1))
  (CallFunction|PrintDebugMessage "[Mod] Player Has left" "(R=0.786458,G=0.000000,B=0.062841,A=1.000000)" 5.0)
  ;[1 1 1] Search all previously recorded player representations for a matching entry
  (for _array_element (Variables|PlayerRepresentations|GetTTTPlayerRepresentation) ; Search all player representations
    (if (== leavingPlayerController (Variables|/Script/KillerJimModProxy.KJModPlayerProxy|GetplayerController _array_element)) ; this entry matches the player leaving...
      ;[1 1 1] If we died, there's a dead pawn (which someone may have scanned) lying in the level, remove it..
      (Utilities|IsValid (Variables|/Game/CustomContent/UGC2164905560/Blueprints/PlayerRepresentation/KJModTTTPlayerBP.KJModTTTPlayerBP_C|GetDeadPawn _array_element)
        (:Is%20Valid
          (Class|KJModPlayerProxy|RemoveDeadPawn _array_element (Variables|/Game/CustomContent/UGC2164905560/Blueprints/PlayerRepresentation/KJModTTTPlayerBP.KJModTTTPlayerBP_C|GetDeadPawn _array_element)))
        (:Is%20Not%20Valid
          _))
      ;[1 1 1] They are dead to us..
      (PlayerManagement|HandlePlayerDeath _array_element)
      ;[1 1 1] Destroy and remove..
      (Actor|DestroyActor _array_element) ; Destroy it
      (Utilities|Array|RemoveItem (Variables|PlayerRepresentations|GetTTTPlayerRepresentation) _array_element) ; Remove from array
      (return false) ; No errors
    ))
  (CallFunction|PrintDebugMessage "[Mod] Could not find the leaving player!!!!" "(R=0.786458,G=0.000000,B=0.062841,A=1.000000)" 25.0)
  (return true) ; Should never reach here!
)

(fn SwitchtoNewState
  (params (State :type KJModTTTGameStateEnum%20Enum :default "NewEnumerator0"))
  ;[1 1 1] Called only when entering a "new" state, so performs one time only set-up for the new state
  (bind _output_get (Variables|GameState|SetState State))
  (CallFunction|PrintDebugMessage (Utilities|String|Append "[Mod] Switching to new state: " (Utilities|String|EnumtoString _output_get)) "(R=0.601397,G=0.567708,B=1.000000,A=1.000000)" 5.0)
  (switch Utilities|FlowControl|Switch|SwitchonKJModTTTGameStateEnum State
    (:NewEnumerator3
      ;[1 1 1] Entering pregame - spawn all players
      (for _array_element (Variables|PlayerRepresentations|GetTTTPlayerRepresentation)
        (Class|KJModGameModeProxy|SpawnPlayer _array_element)
        ;[1 1 1] Set type to "unknown" (shows "Preparing" on local UI of that player as this is RepNot-ified out)
        (Variables|/Game/CustomContent/UGC2164905560/Blueprints/PlayerRepresentation/KJModTTTPlayerBP.KJModTTTPlayerBP_C|SetPlayerType _array_element "NewEnumerator0")
        ;[1 1 1] Reset credits
        (Variables|/Game/CustomContent/UGC2164905560/Blueprints/PlayerRepresentation/KJModTTTPlayerBP.KJModTTTPlayerBP_C|SetPlayerCredits _array_element 0) ; Important; if this value does not change when players are spawned the REPNotify is never called (and they get locally never set their credits). So reset to zero
        ;[1 1 1] Turn off global chat as we're in game
        (Default|SetGlobalChatActive _array_element false)
        ;[1 1 1] Show how long this phase lasts (uses a "owning client" event)
        (Default|SetPhaseTime _array_element (+ (Variables|GameSettings(Editthese)|GetPreroundTime) 5))))
    (:NewEnumerator4
      ;[1 1 1] Game is starting, select who's innocent, traitor and detective (assuming players number allow)
      (PlayerTypeSelection|SelectPlayerTypes))
    (:NewEnumerator5
      ;[1 1 1] Game main phase
      (for _array_element_2 (Variables|PlayerRepresentations|GetTTTPlayerRepresentation)
        (Default|SetPhaseTime _array_element_2 (Variables|GameSettings(Editthese)|GetMainRoundTime))
        (Variables|/Game/CustomContent/UGC2164905560/Blueprints/PlayerRepresentation/KJModTTTPlayerBP.KJModTTTPlayerBP_C|SetGameInPlay _array_element_2 true) ; Game is running (equipment available, for example)
      )
      (Class|KJModGameModeProxy|RoundReset) ; Call round reset, this allows WeaponitemSpawnActors (that the user-choosen level may have) to respawn guns, items, etc.
    )
    (:NewEnumerator6
      ;[1 1 1] Game winner phase
      (for _array_element_3 (Variables|PlayerRepresentations|GetTTTPlayerRepresentation)
        (CallFunction|GenerateRoundReport _array_element_3)
        (Default|SetGlobalChatActive _array_element_3 true)
        (Variables|/Game/CustomContent/UGC2164905560/Blueprints/PlayerRepresentation/KJModTTTPlayerBP.KJModTTTPlayerBP_C|SetGameInPlay _array_element_3 false) ; Game is not running (so no equipment, for example)
      ))
    (:NewEnumerator7
      ;[1 1 1] Round reset; get all clients to remove any round report
      (for _array_element_4 (Variables|PlayerRepresentations|GetTTTPlayerRepresentation)
        (Default|HideRoundReportWidget _array_element_4)
        ;[1 1 1] If we died, there's a dead pawn (which someone may have scanned) lying in the level, remove it..
        (Utilities|IsValid (Variables|/Game/CustomContent/UGC2164905560/Blueprints/PlayerRepresentation/KJModTTTPlayerBP.KJModTTTPlayerBP_C|GetDeadPawn _array_element_4)
          (:Is%20Valid
            (Class|KJModPlayerProxy|RemoveDeadPawn _array_element_4 (Variables|/Game/CustomContent/UGC2164905560/Blueprints/PlayerRepresentation/KJModTTTPlayerBP.KJModTTTPlayerBP_C|GetDeadPawn _array_element_4)))))
      (Class|KJModGameModeProxy|RoundEnd))))

(fn HandleGameReset
  (CallFunction|PrintDebugMessage "[Mod State] Game Reset Called" "(R=0.431641,G=0.479585,B=0.609375,A=1.000000)" 5.0)
  (Utilities|FlowControl|Sequence
    (:then_0
      (Variables|GameState-Pregame|SetPregameTimeout (Variables|GameSettings(Editthese)|GetPreroundTime))
      (Variables|GameState-Pregame|SetPregameLockOutTimeout 5) ; Always 5 seconds of lock out for joining players
    )
    (:then_1
      (Variables|GameState-Main|SetMainRoundTimeout (Variables|GameSettings(Editthese)|GetMainRoundTime)))
    (:then_2
      (Variables|GameState-WinnerPhase|SetWinnerPhaseTimeout (Variables|GameSettings(Editthese)|GetWinnerPhaseTime)))
    (:then_3
      (Variables|GameState-WinnerPhase|SetWinnerType "NewEnumerator1") ; Assume innocents win (if main phase times out)
    )
    (:then_4
      (Class|KJModGameModeProxy|RoundEnd) ; The level designers may have placed world spawn items around and they automatically spawn things on level load. For TTT we don't actual spawn things until we're got enough players; so remove all guns whilst we wait.. (we will respawn later)
    )
    (:then_5
      (StateManagement|SwitchtoNewState "NewEnumerator2") ; After reset, make sure enough players to start a new round
    )))

(fn HandleSelectionState
  (CallFunction|PrintDebugMessage "[Mod State] Selection state, selecting player types" "(R=0.512804,G=0.550874,B=0.708333,A=1.000000)" 5.0)
  (StateManagement|SwitchtoNewState "NewEnumerator5"))

(fn HandleMainPhase
  (CallFunction|PrintDebugMessage (Utilities|String|Append "[Mod State] Main state, timeout: " (Utilities|String|ToString(Integer) (Variables|GameState-Main|GetMainRoundTimeout))) "(R=0.478516,G=0.493503,B=0.656250,A=1.000000)" 5.0)
  (bind _result (Math|Integer|DecrementInt (Variables|GameState-Main|GetMainRoundTimeout))
    (:%20%20
      (bind _output_get (Variables|GameState-Main|SetMainRoundTimeout _result))
      (if (== _output_get 0)
        (StateManagement|SwitchtoNewState "NewEnumerator6")))))

(fn HandleWinnerPhase
  (CallFunction|PrintDebugMessage (Utilities|String|Append "[Mod State] winner state, timeout: " (Utilities|String|ToString(Integer) (Variables|GameState-WinnerPhase|GetWinnerPhaseTimeout))) "(R=0.524089,G=0.609394,B=0.729167,A=1.000000)" 5.0)
  (bind _result (Math|Integer|DecrementInt (Variables|GameState-WinnerPhase|GetWinnerPhaseTimeout))
    (:%20%20
      (bind _output_get (Variables|GameState-WinnerPhase|SetWinnerPhaseTimeout _result))
      (if (== _output_get 0)
        (StateManagement|SwitchtoNewState "NewEnumerator7")))))

(fn HandlePregameLockoutState
  (CallFunction|PrintDebugMessage (Utilities|String|Append "[Mod State] LOCKOUT state, timeout: " (Utilities|String|ToString(Integer) (Variables|GameState-Pregame|GetPregameLockOutTimeout))) "(R=0.518392,G=0.647530,B=0.677083,A=1.000000)" 5.0)
  (bind _result (Math|Integer|DecrementInt (Variables|GameState-Pregame|GetPregameLockOutTimeout))
    (:%20%20
      (bind _output_get (Variables|GameState-Pregame|SetPregameLockOutTimeout _result))
      (if (== _output_get 0)
        (StateManagement|SwitchtoNewState "NewEnumerator4")))))

(fn SelectPlayerTypes
  (bind _returnvalue (Class|KJModGameModeProxy|GetPlayerProxies))
  (CallFunction|PrintDebugMessage (Utilities|String|Append "SelectPlayerTypes called, count: " (Utilities|String|ToString(Integer) (Utilities|Array|Length (Variables|PlayerRepresentations|GetTTTPlayerTypes))) "..and.." (Utilities|String|ToString(Integer) (Utilities|Array|Length _returnvalue))) "(R=0.854167,G=0.000000,B=0.290491,A=1.000000)" 25.0)
  ;[1 1 1] Store locally for ease of access..
  (bind _returnvalue_2 (Class|KJModGameModeProxy|GetPlayerProxies))
  (bind _output_get (LocalVariables|SetPlayerProxies _returnvalue_2))
  (LocalVariables|SetTotalPlayers (Utilities|Array|Length _output_get))
  ;[0 1 0.03257] Clear main struct holding who's who
  (Utilities|Array|Clear (Variables|PlayerRepresentations|GetTTTPlayerTypes))
  ;[1 1 1] Fill player type array with "innocent" for all players joined
  (Utilities|Array|Clear (LocalVariables|GetPlayerTypes))
  (for _array_element (LocalVariables|GetPlayerProxies)
    (Utilities|Array|Add (LocalVariables|GetPlayerTypes) "NewEnumerator1"))
  ;[1 1 1] More than three players? we can make detective
  (if (> (Utilities|Array|Length (LocalVariables|GetPlayerProxies)) 2)
    ;[0.211 1 0.3731] Three or more players
    (Development|PrintString "Three or or more players" true true "(R=1.000000,G=0.830574,B=0.000000,A=1.000000)" 12.0)
    ;;[1 1 1] Detective? If over min player count, then Min 1 to X %
    (if (>= (LocalVariables|GetTotalPlayers) (Variables|GameSettings(Editthese)|GetMinPlayerForDetective))
      (LocalVariables|SetTotalDetectives (Math|Float|Floor (Math|Float|Max(Float) (* (Math|Conversions|ToFloat(Integer) (LocalVariables|GetTotalPlayers)) (Variables|GameSettings(Editthese)|GetDetectiveRatio)) 1.0)))
      (else
        (LocalVariables|SetTotalDetectives 0)))
    ;;[1 1 1] Terrorists? Min 1 to X %
    (LocalVariables|SetTotalTerrorists (Math|Float|Floor (Math|Float|Max(Float) (* (Math|Conversions|ToFloat(Integer) (LocalVariables|GetTotalPlayers)) (Variables|GameSettings(Editthese)|GetTerroristRatio)) 1.0)))
    ;[0.07297 1 0] Select random (but unique) Detectives (1 or more..)
    (Utilities|Array|Clear (LocalVariables|GetPreviouslySelectedIndices))
    (for _index (range 0 (- (LocalVariables|GetTotalDetectives) 1))
      (bind _uniquevalue (PlayerTypeSelection|SelectUniqueRandomValue (LocalVariables|GetPreviouslySelectedIndices) (- (LocalVariables|GetTotalPlayers) 1)))
      (Utilities|Array|Add (LocalVariables|GetPreviouslySelectedIndices) _uniquevalue)
      (Utilities|Array|SetArrayElem (LocalVariables|GetPlayerTypes) _uniquevalue "NewEnumerator3"))
    ;[1 0.8781 0.2304] Select random (but unique) Detectives (1 or more)
    (for _index_2 (range 0 (- (LocalVariables|GetTotalTerrorists) 1))
      (bind _uniquevalue_2 (PlayerTypeSelection|SelectUniqueRandomValue (LocalVariables|GetPreviouslySelectedIndices) (- (LocalVariables|GetTotalPlayers) 1)))
      (Utilities|Array|Add (LocalVariables|GetPreviouslySelectedIndices) _uniquevalue_2)
      (Utilities|Array|SetArrayElem (LocalVariables|GetPlayerTypes) _uniquevalue_2 "NewEnumerator2"))
    (else
      ;[0.9776 1 0.3756] Two players? Not a great game but let's make someone a T
      (Utilities|Array|SetArrayElem (LocalVariables|GetPlayerTypes) (Math|Random|RandomIntegerinRange 0 1) "NewEnumerator2")))
  ;[1 0.739 0.2663] DEBUG (disabled) - output the actual selections for validation (used during development)
  (for (_array_element_2 _array_index) (LocalVariables|GetPlayerTypes)
    (CallFunction|PrintDebugMessage (Utilities|String|Append "Player Index: " (Utilities|String|ToString(Integer) _array_index) " is of type: " (Utilities|String|EnumtoString _array_element_2)) "(R=1.000000,G=0.230251,B=0.000000,A=1.000000)" 25.0))
  ;[1 1 1] Clear any values we are going to now compute
  (Variables|GameState-WinnerPhase|SetTotalTerriroistsInRound 0)
  (Variables|GameState-WinnerPhase|SetTotalPlayersInRound 0)
  ;[1 1 1] Copy the choosen types to the actual players (which are REPNOTified about it)
  (for (_array_element_3 _array_index_2) (LocalVariables|GetPlayerProxies)
    (bind _askjmod_tttplayer_bp (Utilities|Casting|CastToKJModTTTPlayerBP _array_element_3))
    (Variables|/Game/CustomContent/UGC2164905560/Blueprints/PlayerRepresentation/KJModTTTPlayerBP.KJModTTTPlayerBP_C|SetPlayerType _askjmod_tttplayer_bp (Utilities|Array|Get(acopy) (LocalVariables|GetPlayerTypes) _array_index_2))
    ;[0.000554 1 0] Add to the "whos who" structure, so we can track the dead
    (Utilities|Array|Add (Variables|PlayerRepresentations|GetTTTPlayerTypes) (Utilities|Struct|MakePlayerTypesStruct _askjmod_tttplayer_bp (Variables|/Script/KillerJimModProxy.KJModPlayerProxy|GetplayerController _askjmod_tttplayer_bp) (Utilities|Array|Get(acopy) (LocalVariables|GetPlayerTypes) _array_index_2) true))
    (CallFunction|PrintDebugMessage "Added user to TTT type.." "(R=0.854167,G=0.000000,B=0.290491,A=1.000000)" 25.0)
    ;[1 1 1] Record "end of round" stats
    (switch Utilities|FlowControl|Switch|SwitchonKJModTTTPlayerType (Utilities|Array|Get(acopy) (LocalVariables|GetPlayerTypes) _array_index_2)
      (:NewEnumerator1
        _)
      (:NewEnumerator2
        (Variables|GameState-WinnerPhase|SetTotalTerriroistsInRound (+ (Variables|GameState-WinnerPhase|GetTotalTerriroistsInRound) 1)))
      (:NewEnumerator3
        _))
    (Variables|GameState-WinnerPhase|SetTotalPlayersInRound (+ (Variables|GameState-WinnerPhase|GetTotalPlayersInRound) 1))))

(fn GenerateRoundReport
  (params (PlayerProxy :type KJ%20Mod%20TTT%20Player%20BP%20Object%20Reference))
  (Default|ShowRoundReportWidget PlayerProxy (Variables|GameState-WinnerPhase|GetWinnerType) (Variables|GameState-WinnerPhase|GetTotalPlayersInRound) (Variables|GameState-WinnerPhase|GetTotalTerriroistsInRound) (- (Variables|GameSettings(Editthese)|GetMainRoundTime) (Variables|GameState-Main|GetMainRoundTimeout)) "<bold>Post game report</> 
 
In the future we might even add some information here about the state of player. "))

(fn HandlePlayerDeath
  (params (DeadPlayer :type KJ%20Mod%20TTT%20Player%20BP%20Object%20Reference))
  ;[1 1 1] Only care about main phase deaths..
  (if (Utilities|Enum|Equal(Enum) (Variables|GameState|GetState) "NewEnumerator5")
    (CallFunction|PrintDebugMessage (Utilities|String|Append "[KJModTTTGameModeBP] HandlePlayerDeath, players: " (Utilities|String|ToString(Integer) (Utilities|Array|Length (Variables|PlayerRepresentations|GetTTTPlayerTypes)))) "(R=0.296247,G=1.000000,B=0.000000,A=1.000000)" 25.0)
    ;[1 1 1] Scan all the "whos who" player array for a matching player proxy
    (bind (_array_element _array_index) (Utilities|Array|ForEachLoopwithBreak (Variables|PlayerRepresentations|GetTTTPlayerTypes) :!label _label)
      (:LoopBody
        ;[1 1 1] Match?
        (if (== (Utilities|Struct|BreakPlayerTypesStruct _array_element) DeadPlayer)
          ;[1 1 1] Mark player as DEAD, and break loop
          (bind _structout (Utilities|Struct|SetmembersinPlayerTypesStruct _array_element false))
          (Utilities|Array|SetArrayElem (Variables|PlayerRepresentations|GetTTTPlayerTypes) _array_index _structout)
          (goto _label Break)))
      (:Completed
        ;[0 0.7732 1] Detect any innocent (or detectives) still alive
        (LocalVariables|SetbAnyInnocentAlive false)
        (bind _array_element_2 (Utilities|Array|ForEachLoopwithBreak (Variables|PlayerRepresentations|GetTTTPlayerTypes) :!label _label_2)
          (:LoopBody
            (if (and (or (Utilities|Enum|Equal(Enum) (.PlayerType (Utilities|Struct|BreakPlayerTypesStruct _array_element_2)) "NewEnumerator1") (Utilities|Enum|Equal(Enum) (.PlayerType (Utilities|Struct|BreakPlayerTypesStruct _array_element_2)) "NewEnumerator3")) (.Alive (Utilities|Struct|BreakPlayerTypesStruct _array_element_2)))
              (LocalVariables|SetbAnyInnocentAlive true)
              (goto _label_2 Break)))
          (:Completed
            ;[0.3073 0.01388 0.04759] Detect any traitors still alive
            (LocalVariables|SetbAnyTraitorsAlive false)
            (bind _array_element_3 (Utilities|Array|ForEachLoopwithBreak (Variables|PlayerRepresentations|GetTTTPlayerTypes) :!label _label_3)
              (:LoopBody
                (if (and (Utilities|Enum|Equal(Enum) (.PlayerType (Utilities|Struct|BreakPlayerTypesStruct _array_element_3)) "NewEnumerator2") (.Alive (Utilities|Struct|BreakPlayerTypesStruct _array_element_3)))
                  (LocalVariables|SetbAnyTraitorsAlive true)
                  (goto _label_3 Break)))
              (:Completed
                ;[1 1 1] Innocents Win?
                (if (and (LocalVariables|GetbAnyInnocentAlive) (not (LocalVariables|GetbAnyTraitorsAlive)))
                  (Variables|GameState-WinnerPhase|SetWinnerType "NewEnumerator1")
                  (StateManagement|SwitchtoNewState "NewEnumerator6")
                  (else
                    ;[1 1 1] Traitors win?
                    (if (and (not (LocalVariables|GetbAnyInnocentAlive)) (LocalVariables|GetbAnyTraitorsAlive)) ; False? game still going
                      (Variables|GameState-WinnerPhase|SetWinnerType "NewEnumerator2")
                      (StateManagement|SwitchtoNewState "NewEnumerator6")
                      (else
                        (CallFunction|PrintDebugMessage "[KJModTTTGameModeBP] HandlePlayerDeath - no overall winner, game still running.." "(R=0.131881,G=1.000000,B=0.000000,A=1.000000)" 1e+01)
                        (bind (_array_element_4 _array_index_2) (Utilities|Array|ForEachLoopwithBreak (Variables|PlayerRepresentations|GetTTTPlayerTypes))
                          (:LoopBody
                            (CallFunction|PrintDebugMessage (Utilities|String|Append "Player ID: " (Utilities|String|ToString(Integer) _array_index_2) ", Settings:" (Utilities|String|Append (Utilities|GetDisplayName (.TTTPlayerProxy (Utilities|Struct|BreakPlayerTypesStruct _array_element_4))) " - " (Utilities|GetDisplayName (.Controller (Utilities|Struct|BreakPlayerTypesStruct _array_element_4))) " = " (Utilities|String|EnumtoString (.PlayerType (Utilities|Struct|BreakPlayerTypesStruct _array_element_4))) " / " (Utilities|String|ToString(Boolean) (.Alive (Utilities|Struct|BreakPlayerTypesStruct _array_element_4))) " ...")) "(R=0.131881,G=1.000000,B=0.000000,A=1.000000)" 15.0)))))))))))))))

(fn ShowInformationtoAllPlayers
  (params (Visible :type Boolean) (Message%20 :type String))
  ;[1 1 1] Show a messsage to players, visible = false causes empty message to be sent (which causes client to hide message)
  (bind _returnvalue (Class|KJModGameModeProxy|GetPlayerProxies))
  (for _array_element _returnvalue
    (bind _askjmod_tttplayer_bp (Utilities|Casting|CastToKJModTTTPlayerBP _array_element))
    (Variables|/Game/CustomContent/UGC2164905560/Blueprints/PlayerRepresentation/KJModTTTPlayerBP.KJModTTTPlayerBP_C|SetHeadlineInformation _askjmod_tttplayer_bp (select Visible Message%20 ""))))

(fn SelectUniqueRandomValue
  (params (PreviousValues :type Array%20of%20Integers) (MaxValue :type Integer))
  (LocalVariables|SetMaxIterations 32) ; Incase someone configures the ratio's wrong, we limit it to 32 (max players)
  (LocalVariables|SetUniqueValueFound false)
  (while (and (not (LocalVariables|GetUniqueValueFound)) (> (LocalVariables|GetMaxIterations) 0))
    (bind _output_get (LocalVariables|SetUniqueNumber (Math|Random|RandomIntegerinRange 0 MaxValue)))
    (if (== (Utilities|Array|FindItem PreviousValues _output_get) -1)
      (LocalVariables|SetUniqueValueFound true)
      (else
        (Math|Integer|DecrementInt (LocalVariables|GetMaxIterations)))))
  (return (LocalVariables|GetUniqueNumber)))

(fn CheckEnoughPlayers
  (if (< (Variables|GameState|GetCurrentPlayerCount) (Variables|GameSettings(Editthese)|GetMinPlayers))
    (StateManagement|SwitchtoNewState "NewEnumerator7")))