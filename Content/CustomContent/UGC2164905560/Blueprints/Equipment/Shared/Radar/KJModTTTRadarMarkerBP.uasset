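; Radar marker actor for a TTT mod that marks a player with a role-colored plane and a distance readout.
; On BeginPlay it creates a dynamic material, and a timeline fades the plane and text before destroying the actor.
; Each tick it turns horizontally toward the local camera, scales up with distance and displays meters.
; It destroys itself early if the linked player proxy is invalid or dead.
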(event EventBeginPlay
  (bind _playertype (Variables|Default|GetPlayerType))
  (bind _returnvalue (Utilities|Select :Index _playertype :NewEnumerator0 "(R=1.000000,G=0.998224,B=0.000000,A=1.000000)" :NewEnumerator1 "(R=0.000000,G=1.000000,B=0.046985,A=1.000000)" :NewEnumerator2 "(R=0.042671,G=1.000000,B=0.000000,A=1.000000)" :NewEnumerator3 "(R=0.072169,G=0.000000,B=1.000000,A=1.000000)"))
  (bind (_r _g _b) (Math|Color|BreakColor _returnvalue))
  ;[0.439 1 0.2816] BEGIN PLAY - Over 25 seconds (using a time-line) fade out the circle and eventually kill it
  (bind _returnvalue_2 (Rendering|Material|CreateDynamicMaterialInstance (Variables|Default|GetRadarMarkerPlane) 0 "/Game/CustomContent/UGC2164905560/Materials/RadarTargetMat.RadarTargetMat" "None" :!class /Script/Engine.PrimitiveComponent))
  (Variables|Default|SetDynamicMaterial _returnvalue_2)
  (bind _opacityfade (Timeline|FadeOverTime PlayFromStart)
    (:Update
      (Rendering|Material|SetVectorParameterValue (Variables|Default|GetDynamicMaterial) "Color" (Math|Color|MakeColor _r _g _b _opacityfade) :!class /Script/Engine.MaterialInstanceDynamic)
      (Rendering|Components|TextRender|SetTextRenderColor (Variables|Default|GetDistanceTextRender) (Math|Conversions|ToColor(LinearColor) (Math|Color|MakeColor _r _g _b _opacityfade) false)))
    (:Finished
      (Actor|DestroyActor))))

(event EventTick
  (params (DeltaSeconds :type Float%20%28single-precision%29))
  (bind _returnvalue (Game|GetPlayerCameraManager 0))
  (bind _returnvalue_2 (Transformation|GetActorLocation))
  (bind _returnvalue_3 (Camera|GetCameraLocation _returnvalue))
  (bind (_x _y) (Math|Vector|BreakVector _returnvalue_2))
  (bind (_x_2 _y_2) (Math|Vector|BreakVector _returnvalue_3))
  (bind _returnvalue_4 (Math|Vector|MakeVector _x _y 0.0))
  (bind _returnvalue_5 (Math|Vector|MakeVector _x_2 _y_2 0.0))
  (bind _returnvalue_6 (- _returnvalue_4 _returnvalue_5))
  (bind _returnvalue_7 (Math|Vector|VectorLength _returnvalue_6))
  ;[1 1 1] EVENT TICK - Make sure the radar marker always faces the player
  (Utilities|IsValid (Variables|Default|GetPlayerProxy) ; Player left?
    (:Is%20Valid
      (if (Variables|/Game/CustomContent/UGC2164905560/Blueprints/PlayerRepresentation/KJModTTTPlayerBP.KJModTTTPlayerBP_C|GetIsPlayerDead (Variables|Default|GetPlayerProxy)) ; Player dead?
        ;[1 0.1453 0.1751] The player we're linked to is dead, we're no longer needed
        (Actor|DestroyActor :!label _label)
        (else
          (Transformation|SetActorRotation (Math|Rotator|FindLookatRotation _returnvalue_4 _returnvalue_5) true) ; Rotate us to face the local camera (player)
          (Transformation|SetActorScale3D (Math|Conversions|ToVector(Float) (Math|Float|Max(Float) (/ _returnvalue_7 1e+03) 1.0))) ; Ensure we never shrink too much
          ;[1 1 1] Show distance on text renderer
          (Rendering|Components|TextRender|SetText (Variables|Default|GetDistanceTextRender) (Utilities|Text|ToText(Float) (/ _returnvalue_7 1e+02) "HalfToEven" false false 1 324 0 1)))))
    (:Is%20Not%20Valid
      (goto _label))))

(fn ConstructionScript)